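; Game mode for a Diablo-like top-down game that builds a procedural dungeon at BeginPlay behind a loading screen.
; A Spelunky-style wander generates the layout, which a spawned DungeonSpawner builds from the forest tileset; an older hand-built test layout is unused.
; OnLevelsLoaded moves the player to the start column, enables gravity, removes the loading screen, spawns the goal and shows instructions.
; PercentLevelsLoaded passes through the spawner's load progress.
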(event `self.ReceiveBeginPlay`
  (bind _dungeonspawner (`self.DungeonSpawner`))
  (`self.CreateLoadingScreen`)
  (`self.CreateDungeonSpawner`)
  (bind _dungeon (`self.MakeTestDungeon`))
  (`KismetSystemLibrary.PrintString` "Dungeon Made")
  (`DungeonSpawner.SetDungeon` _dungeonspawner _dungeon)
  (`DungeonSpawner.SpawnDungeon` _dungeonspawner (0.0 0.0 0.0) true))

(fn `CreateDungeonSpawner`
  (bind _returnvalue (`|SpawnActorFromClass` "/Game/Blueprints/DungeonSpawner_BP.DungeonSpawner_BP_C" (`KismetMathLibrary.MakeTransform` (0.0 0.0 0.0)) "Undefined" "OverrideRootScale" null null))
  (bind _output_get (set `self.DungeonSpawner` _returnvalue))
  (set `DungeonSpawner.Tileset` "/Game/Levels/Tilesets/ForestTileset.ForestTileset" _output_get)
  (set `DungeonSpawner.TileSize` 1000.0 _output_get))

(fn `CreateLoadingScreen`
  (bind _returnvalue (`|CreateWidget` "/Game/Blueprints/LoadingScreen.LoadingScreen_C" (`GameplayStatics.GetPlayerController` 0)))
  (bind _output_get (set `self.Loading Screen` _returnvalue))
  (`UserWidget.AddToPlayerScreen` _output_get 0))

(fn `MakeTestDungeon`
  (returns (Dungeon :type "GenericDungeon Object Reference"))
  (locals (newDungeon :type "GenericDungeon Object Reference"))
  (bind _dungeon (`SimpleDungeonDesigner.SpelunkyWander` 5))
  (bind _output_get (set `self.Dungeon` _dungeon))
  (return _output_get))

(fn `On Levels Loaded`
  (params (TileSize :type "Float (double-precision)"))
  (bind _loading_screen (`self.Loading Screen`))
  (bind (_x _y) (`GenericDungeon.GetGoalTile` (`self.Dungeon`)))
  (bind _astop_down_character (cast `/Game/TopDownCPP/Blueprints/TopDownCharacter` (`Controller.K2_GetPawn` (`GameplayStatics.GetPlayerController` 0)))
    (:`then`
      (`self.K2_SetActorLocation` _astop_down_character (`KismetMathLibrary.MakeVector` (* (`GenericDungeon.GetStartTile` (`self.Dungeon`)) TileSize) 0.0 120.0) false false)
      (`/Game/TopDownCPP/Blueprints/TopDownCharacter.EnableGravity` _astop_down_character)
      (`/Engine/EditorBlueprintResources/StandardMacros.IsValid` _loading_screen
        (:`Is Valid`
          (`Widget.RemoveFromParent` _loading_screen))
        (:`Is Not Valid`
          _)))
    (:`CastFailed`
      _))
  (`|SpawnActorFromClass` "/Game/Blueprints/Props/LevelGoal.LevelGoal_C" (`KismetMathLibrary.MakeTransform` (`KismetMathLibrary.MakeVector` (* _x TileSize) (* _y TileSize) 30.0)) "Undefined" "OverrideRootScale" null null)
  (bind _returnvalue (`|CreateWidget` "/Game/Blueprints/Instruction.Instruction_C"))
  (`UserWidget.AddToPlayerScreen` _returnvalue 0))

(fn `PercentLevelsLoaded`
  (returns (Percentage :type "Float (double-precision)"))
  (return (`DungeonSpawner.PercentLevelsLoaded` (`self.DungeonSpawner`))))

(fn `UserConstructionScript`)
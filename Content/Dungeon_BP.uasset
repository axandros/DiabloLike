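; Dungeon Blueprint that stores a grid map of tiles along with its width, height, start tile and goal tile.
; Tiles live in one flat array, addressed by converting X/Y to an index with X times width plus Y.
; Getters and setters read and write tiles, resize the array and set start and goal after index checks.
; Out-of-bounds reads return a generic tile and a flag.
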(fn `ConvertCoordinatesToInt`
  (params (X :type Integer) (Y :type Integer))
  (returns (Index :type Integer))
  (return (+ Y (* X (`self.DungeonWidth`)))))

(fn `ConvertIntToCoordinates`
  (params (Index :type Integer))
  (returns (X :type Integer) (Y :type Integer))
  (bind _dungeonwidth (`self.DungeonWidth`))
  (return (/ Index _dungeonwidth) (mod Index _dungeonwidth)))

(fn `Dimensions`
  (returns (Width :type Integer) (Height :type Integer))
  (return (`self.DungeonWidth`) (`self.DungeonHeight`)))

(fn `GetTile`
  (params (X :type Integer) (Y :type Integer))
  (returns (Tile :type "GenericTile Structure") (OutOfBounds :type Boolean))
  (bind _out_of_bounds (`self.IsOutOfBounds` X Y))
  (if _out_of_bounds
    (return (make `GenericTile` false) _out_of_bounds)
    (else
      (return (`|GetArrayItem` (`self.DungeonArray`) (`self.ConvertCoordinatesToInt` X Y)) _out_of_bounds))))

(fn `GetTileArray`
  (returns (NewParam :type "Array of GenericTile Structure"))
  (return (`self.DungeonArray`)))

(fn `Goal Tile`
  (returns (X :type Integer) (Y :type Integer))
  (bind __endtile (`self._EndTile`))
  (return (`|GetArrayItem` __endtile) (`|GetArrayItem` __endtile 1)))

(fn `IsOutOfBounds`
  (params (X :type Integer) (Y :type Integer))
  (returns (`Out of Bounds` :type Boolean))
  (bind _index (`self.ConvertCoordinatesToInt` X Y))
  (bind (_width _height) (`self.Dimensions`))
  (return (not (and (<= _index (`self.ConvertCoordinatesToInt` _width _height)) (>= _index 0)))))

(fn `SetDungeonDimensions`
  (params (Width :type Integer) (Height :type Integer))
  (returns (Successful :type Boolean))
  (bind _output_get (set `self.DungeonWidth` Width))
  (bind _output_get_2 (set `self.DungeonHeight` Height))
  (`KismetArrayLibrary.Array_Resize` (`self.DungeonArray`) (* _output_get_2 _output_get))
  (return true))

(fn `SetGoalTile`
  (params (X :type Integer) (Y :type Integer))
  (returns (`Successfully Set` :type Boolean))
  (bind _index (`self.ConvertCoordinatesToInt` X Y))
  (bind __endtile (`self._EndTile`))
  (bind _returnvalue (and (< _index (`KismetArrayLibrary.Array_Length` (`self.DungeonArray`))) (>= _index 0) (< Y (`self.DungeonWidth`)) (< X (`self.DungeonHeight`))))
  (if _returnvalue
    (`KismetArrayLibrary.Array_Set` __endtile 0 X true)
    (`KismetArrayLibrary.Array_Set` __endtile 1 Y true))
  (return _returnvalue))

(fn `SetStartTile`
  (params (X :type Integer) (Y :type Integer))
  (returns (`Successfully Set` :type Boolean))
  (bind _index (`self.ConvertCoordinatesToInt` X Y))
  (bind __starttile (`self._StartTile`))
  (bind _returnvalue (and (< _index (`KismetArrayLibrary.Array_Length` (`self.DungeonArray`))) (>= _index 0)))
  (if _returnvalue
    (`KismetArrayLibrary.Array_Set` __starttile 0 X true)
    (`KismetArrayLibrary.Array_Set` __starttile 1 Y true))
  (return _returnvalue))

(fn `SetTile`
  (params (X :type Integer) (Y :type Integer) (Tile :type "GenericTile Structure"))
  (if (not (`self.IsOutOfBounds` X Y))
    (`KismetArrayLibrary.Array_Set` (`self.DungeonArray`) (`self.ConvertCoordinatesToInt` X Y) Tile true))
  (return))

(fn `Start Tile`
  (returns (X :type Integer) (Y :type Integer))
  (bind __starttile (`self._StartTile`))
  (return (`|GetArrayItem` __starttile) (`|GetArrayItem` __starttile 1)))
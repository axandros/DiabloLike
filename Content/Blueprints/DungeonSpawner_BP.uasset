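; Dungeon spawner actor that turns grid tiles into streamed level instances to build the dungeon.
; SpawnTile maps each non-void tile's North/South/East/West exits to the first level in the matching Tileset array.
; It loads that level at a grid offset scaled by TileSize, tracks it and binds its loaded event.
; A completion check notifies DiabloLikeGameMode_BP with the tile size once all levels are loaded.
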(event `self.AllLevelsLoaded`)

(event `self.SpawnTile`
  (params (tile :type "GenericTile Structure") (gridX :type Integer) (gridY :type Integer))
  (bind (_north _south _east _west _void) (break `GenericTile` tile))
  (bind _tileset (`self.Tileset`))
  (bind _tileset_2 (`self.Tileset`))
  (bind _tilesize (`self.TileSize`))
  (bind _tileset_3 (`self.Tileset`))
  (bind _tileset_4 (`self.Tileset`))
  (bind _tileset_5 (`self.Tileset`))
  (bind _tileset_6 (`self.Tileset`))
  (bind _tileset_7 (`self.Tileset`))
  (bind _tileset_8 (`self.Tileset`))
  (if (not _void)
    (if _north
      (if _south
        (if _east
          (if _west
            (set `self.Scene to Load` (`|GetArrayItem` (`TilesetAsset.NESW_Tiles` _tileset_8)))
            (else
              (set `self.Scene to Load` (`|GetArrayItem` (`TilesetAsset.NES_Tiles` _tileset_8)))))
          (elif _west
            (set `self.Scene to Load` (`|GetArrayItem` (`TilesetAsset.NSW_Tiles` _tileset_7)))
            (else
              (set `self.Scene to Load` (`|GetArrayItem` (`TilesetAsset.NS_Tiles` _tileset_7))))))
        (elif _east
          (if _west
            (set `self.Scene to Load` (`|GetArrayItem` (`TilesetAsset.NEW_Tiles` _tileset_6)))
            (else
              (set `self.Scene to Load` (`|GetArrayItem` (`TilesetAsset.NE_Tiles` _tileset_6)))))
          (elif _west
            (set `self.Scene to Load` (`|GetArrayItem` (`TilesetAsset.NW_Tiles` _tileset_5)))
            (else
              (set `self.Scene to Load` (`|GetArrayItem` (`TilesetAsset.N_Tiles` _tileset_5)))))))
      (elif _south
        (if _east
          (if _west
            (set `self.Scene to Load` (`|GetArrayItem` (`TilesetAsset.ESW_Tiles` _tileset_4)))
            (else
              (set `self.Scene to Load` (`|GetArrayItem` (`TilesetAsset.ES_Tiles` _tileset_4)))))
          (elif _west
            (set `self.Scene to Load` (`|GetArrayItem` (`TilesetAsset.SW_Tiles` _tileset_3)))
            (else
              (set `self.Scene to Load` (`|GetArrayItem` (`TilesetAsset.S_Tiles` _tileset_3))))))
        (elif _east
          (if _west
            (set `self.Scene to Load` (`|GetArrayItem` (`TilesetAsset.EW_Tiles` _tileset_2)))
            (else
              (set `self.Scene to Load` (`|GetArrayItem` (`TilesetAsset.E_Tiles` _tileset_2)))))
          (elif _west
            (set `self.Scene to Load` (`|GetArrayItem` (`TilesetAsset.W_Tiles` _tileset)))
            (else
              (set `self.Scene to Load` (`|GetArrayItem` (`TilesetAsset.NoExit_Tiles` _tileset))))))))
    (bind (_boutsuccess _returnvalue) (`LevelStreamingDynamic.LoadLevelInstanceBySoftObjectPtr` (`self.Scene to Load`) (+ (`self.SpawnLocation`) (`KismetMathLibrary.MakeVector` (* _tilesize (`KismetMathLibrary.Conv_IntToDouble` gridX)) (* _tilesize (`KismetMathLibrary.Conv_IntToDouble` gridY)))))) ; Made the Dungeon Spawner class inherit from AActor in order to call this.
    (`KismetArrayLibrary.Array_Add` (`self.levelsLoading`) _returnvalue)
    (add `LevelStreaming.OnLevelLoaded` _returnvalue (`|CreateDelegate` :!event `AreAllLevelsLoadedF`))))

(fn `AllLevelsLoadedF`
  (if true
    (bind _asdiablo_like_game_mode_bp (cast `/Game/DiabloLikeGameMode_BP` (`GameplayStatics.GetGameMode`)))
    (`/Game/DiabloLikeGameMode_BP.On Levels Loaded` _asdiablo_like_game_mode_bp (`self.TileSize`))))

(fn `AreAllLevelsLoadedF`
  (locals (`Levels Loaded` :type Boolean))
  (if (`self.AreAllLevelsLoaded`)
    (`self.AllLevelsLoadedF`))
  (return))

(fn `UserConstructionScript`)
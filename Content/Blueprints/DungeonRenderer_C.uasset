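; Actor that builds a random 5x5 dungeon at BeginPlay behind a loading screen, then places the player and level goal.
; A seeded, Spelunky-style random walk carves exits from start to goal in a GenericDungeon grid, then edges are sealed.
; Each tile, plus a closed border ring, streams a random level instance matching its exits.
; Once all levels load, the player is moved, the goal spawned and instructions shown.
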(event `self.ReceiveBeginPlay`
  (bind _returnvalue (`|CreateWidget` "/Game/Blueprints/LoadingScreen.LoadingScreen_C" (`GameplayStatics.GetPlayerController` 0)))
  (set `self.LoadingScreen` _returnvalue)
  (`UserWidget.AddToPlayerScreen` _returnvalue 0)
  (`self.Generate Dungeon`))

(event `All Levels Loaded`
  (bind _tilesize (`self.TileSize`))
  (bind (_x _y) (`GenericDungeon.GetGoalTile` (`self.ActiveDungeon`)))
  (bind _astop_down_character (cast `/Game/TopDownCPP/Blueprints/TopDownCharacter` (`Controller.K2_GetPawn` (`GameplayStatics.GetPlayerController` 0)))
    (:`then`
      (`self.K2_SetActorLocation` _astop_down_character (`KismetMathLibrary.MakeVector` (* (`GenericDungeon.GetStartTile` (`self.ActiveDungeon`)) (`self.TileSize`)) 0.0 120.0) false false)
      (`KismetSystemLibrary.Delay` 1.5)
      (`/Game/TopDownCPP/Blueprints/TopDownCharacter.EnableGravity` _astop_down_character))
    (:`CastFailed`
      _))
  (`Widget.RemoveFromParent` (`self.LoadingScreen`))
  (`|SpawnActorFromClass` "/Game/Blueprints/LevelGoal.LevelGoal_C" (`KismetMathLibrary.MakeTransform` (`KismetMathLibrary.MakeVector` (* _x _tilesize) (* _y _tilesize) 30.0)) "Undefined" "OverrideRootScale" null null)
  (bind _returnvalue (`|CreateWidget` "/Game/Blueprints/Instruction.Instruction_C"))
  (`UserWidget.AddToPlayerScreen` _returnvalue 0))

(fn `AddDungeonToWorld`
  (locals (`Scene to Load` :type "World Soft Object Reference") (`Spawn Location` :type "Vector Structure"))
  (bind _activedungeon (`self.ActiveDungeon`))
  (bind _activedungeon_2 (`self.ActiveDungeon`))
  (bind (_x _y) (`GenericDungeon.GetStartTile` _activedungeon_2))
  (bind (_x_2 _y_2) (`GenericDungeon.GetGoalTile` _activedungeon_2))
  (`KismetSystemLibrary.PrintString` (`KismetStringLibrary.Concat_StrStr` "Start: (" (`KismetStringLibrary.Conv_IntToString` _x) ", " (`KismetStringLibrary.Conv_IntToString` _y) ")   Goal: (" (`KismetStringLibrary.Conv_IntToString` _x_2) ", " (`KismetStringLibrary.Conv_IntToString` _y_2) ")"))
  (for (_array_element _array_index) (`GenericDungeon.GetAllTiles` _activedungeon)
    (bind (_x_3 _y_3) (`GenericDungeon.ConvertIntToCoordinates` _activedungeon _array_index))
    (`self.DebugPrintTile` _array_element _x_3 _y_3
      (:`Out`
        (`self.RenderTile` _x_3 _y_3 _array_element))))
  (return))

(fn `AreAllLevelsLoaded`
  (locals (`Levels Loaded` :type Boolean))
  (set `local.Levels Loaded` true)
  (for _array_element (`self.Levels Loading`)
    (if (not (`LevelStreaming.IsLevelLoaded` _array_element))
      (set `local.Levels Loaded` false)
      (break)))
  (if (`local.Levels Loaded`)
    (`self.All Levels Loaded`))
  (return))

(fn `Generate Dungeon`
  (locals (StartPosition :type "Vector Structure" :default (0.0 0.0 0.0)))
  (`/Engine/EditorBlueprintResources/StandardMacros.IsValid` (`self.ActiveDungeon`)
    (:`Is Valid`
      _)
    (:`Is Not Valid`
      (bind _returnvalue (`|GenericCreateObject` "/Script/DiabloLike.GenericDungeon" self))
      (set `self.ActiveDungeon` _returnvalue)))
  (`GenericDungeon.SetDungeonDimensions` (`self.ActiveDungeon`) 5 5)
  (`self.Spelunky Wander`)
  (`self.Seal Off Dungeon`)
  (`self.SurroundWithClosed`)
  (`self.AddDungeonToWorld`))

(fn `PercentLoadedLevels`
  (returns (Percent :type "Float (double-precision)"))
  (locals (LoadedLevels :type Integer))
  (bind _levels_loading (`self.Levels Loading`))
  (for _array_element _levels_loading
    (if (`LevelStreaming.IsLevelLoaded` _array_element)
      (`/Engine/EditorBlueprintResources/StandardMacros.IncrementInt` (`local.LoadedLevels`))))
  (return (/ (`KismetMathLibrary.Conv_IntToDouble` (`local.LoadedLevels`)) (`KismetMathLibrary.Conv_IntToDouble` (`KismetArrayLibrary.Array_Length` _levels_loading)))))

(fn `RenderTile`
  (params (X :type Integer) (Y :type Integer) (Tile :type "GenericTile Structure"))
  (locals (`Scene to Load` :type "World Soft Object Reference"))
  (bind (_north _south _east _west _void) (break `GenericTile` Tile))
  (bind _tilesize (`self.TileSize`))
  (if _north
    (if _south
      (if _east
        (if _west
          (set `local.Scene to Load` (`self.RandomTile` (`self.NSEW_Tiles`)))
          (else
            (set `local.Scene to Load` (`self.RandomTile` (`self.NSE_Tiles`)))))
        (elif _west
          (set `local.Scene to Load` (`self.RandomTile` (`self.NSW_Tiles`)))
          (else
            (set `local.Scene to Load` (`self.RandomTile` (`self.NS_Tiles`))))))
      (elif _east
        (if _west
          (set `local.Scene to Load` (`self.RandomTile` (`self.NEW_Tiles`)))
          (else
            (set `local.Scene to Load` (`self.RandomTile` (`self.NE_Tiles`)))))
        (elif _west
          (set `local.Scene to Load` (`self.RandomTile` (`self.NW_Tiles`)))
          (else
            (set `local.Scene to Load` (`self.RandomTile` (`self.N_Tiles`)))))))
    (elif _south
      (if _east
        (if _west
          (set `local.Scene to Load` (`self.RandomTile` (`self.SEW_Tiles`)))
          (else
            (set `local.Scene to Load` (`self.RandomTile` (`self.SE_Tiles`)))))
        (elif _west
          (set `local.Scene to Load` (`self.RandomTile` (`self.SW_Tiles`)))
          (else
            (set `local.Scene to Load` (`self.RandomTile` (`self.S_Tiles`))))))
      (elif _east
        (if _west
          (set `local.Scene to Load` (`self.RandomTile` (`self.EW_Tiles`)))
          (else
            (set `local.Scene to Load` (`self.RandomTile` (`self.E_Tiles`)))))
        (elif _west
          (set `local.Scene to Load` (`self.RandomTile` (`self.W_Tiles`)))
          (else
            (set `local.Scene to Load` (`self.RandomTile` (`self.X_Tiles`))))))))
  (bind (_boutsuccess _returnvalue) (`LevelStreamingDynamic.LoadLevelInstanceBySoftObjectPtr` (`local.Scene to Load`) (+ (`self.StartLocation`) (`KismetMathLibrary.MakeVector` (* _tilesize (`KismetMathLibrary.Conv_IntToDouble` X)) (* _tilesize (`KismetMathLibrary.Conv_IntToDouble` Y))))))
  (`KismetArrayLibrary.Array_Add` (`self.Levels Loading`) _returnvalue)
  (add `LevelStreaming.OnLevelLoaded` _returnvalue (`|CreateDelegate` :!event `AreAllLevelsLoaded`))
  (return))

(fn `Seal Off Dungeon`
  (bind _activedungeon (`self.ActiveDungeon`))
  (bind _activedungeon_2 (`self.ActiveDungeon`))
  (bind _activedungeon_3 (`self.ActiveDungeon`))
  (bind _activedungeon_4 (`self.ActiveDungeon`))
  (for _index (range 5)
    (bind (_north _south _east _west _void) (break `GenericTile` (`GenericDungeon.GetTile` _activedungeon_2 _index 0)))
    ;[1 1 1] West Column
    (`GenericDungeon.SetTile` _activedungeon_2 _index 0 (make `GenericTile` _north _south _east false _void))
    (bind (_north_2 _south_2 _east_2 _west_2 _void_2) (break `GenericTile` (`GenericDungeon.GetTile` _activedungeon_3 0 _index)))
    ;[1 1 1] South Row
    (`GenericDungeon.SetTile` _activedungeon_3 0 _index (make `GenericTile` _north_2 false _east_2 _west_2 _void_2))
    (bind (_north_3 _south_3 _east_3 _west_3 _void_3) (break `GenericTile` (`GenericDungeon.GetTile` _activedungeon_4 4 _index)))
    ;[1 1 1] North Row
    (`GenericDungeon.SetTile` _activedungeon_4 4 _index (make `GenericTile` false _south_3 _east_3 _west_3 _void_3))
    (bind (_north_4 _south_4 _east_4 _west_4 _void_4) (break `GenericTile` (`GenericDungeon.GetTile` _activedungeon _index 0)))
    ;[1 1 1] EastColumn
    (`GenericDungeon.SetTile` _activedungeon _index 0 (make `GenericTile` _north_4 _south_4 false _west_4 _void_4)))
  (return))

(fn `Spelunky Wander`
  (locals (X :type Integer) (Y :type Integer) (OOB :type Boolean) (Direction :type String))
  (bind _y (`local.Y`))
  (bind _rng (`self.RNG`))
  (bind _x (`local.X`))
  (bind _y_2 (`local.Y`))
  (bind _x_2 (`local.X`))
  (bind _y_3 (`local.Y`))
  (bind _x_3 (`local.X`))
  (bind _x_4 (`local.X`))
  (bind _y_4 (`local.Y`))
  (bind _returnvalue (not (`local.OOB`)))
  (bind (_year _month _day _hour _minute _second _millisecond) (`KismetMathLibrary.BreakDateTime` (`KismetMathLibrary.Now`)))
  (bind _returnvalue_2 (- _x_2 1))
  (bind _returnvalue_3 (+ _y_2 1))
  (bind _returnvalue_4 (+ _x_4 1))
  (bind (_north _south _east _west) (break `GenericTile` (`GenericDungeon.GetTile` (`self.ActiveDungeon`) _x_2 _y_3)))
  (bind (_north_2 _south_2 _east_2 _west_2) (break `GenericTile` (`GenericDungeon.GetTile` (`self.ActiveDungeon`) _x _y_2)))
  (bind (_north_3 _south_3 _east_3 _west_3) (break `GenericTile` (`GenericDungeon.GetTile` (`self.ActiveDungeon`) _x_4 _y_4)))
  (bind (_tile _returnvalue_5) (`GenericDungeon.GetTile` (`self.ActiveDungeon`) (`local.X`) (+ (`local.Y`) 1)))
  (bind (_north_4 _south_4 _east_4 _west_4) (break `GenericTile` (`GenericDungeon.GetTile` (`self.ActiveDungeon`) _returnvalue_2 _y_3)))
  (bind (_north_5 _south_5 _east_5) (break `GenericTile` (`GenericDungeon.GetTile` (`self.ActiveDungeon`) _x _returnvalue_3)))
  (bind (_north_6 _south_6 _east_6 _west_5) (break `GenericTile` (`GenericDungeon.GetTile` (`self.ActiveDungeon`) _returnvalue_4 _y_4)))
  (bind _asdmap_instance (cast `/Game/Blueprints/DMapInstance` (`GameplayStatics.GetGameInstance`))
    (:`then`
      (bind _seed (`/Game/Blueprints/DMapInstance.GetNextSeed` _asdmap_instance))
      (`KismetSystemLibrary.PrintString` (`KismetStringLibrary.Concat_StrStr` "SEED: " (`KismetStringLibrary.Conv_IntToString` _seed)))
      (`KismetMathLibrary.SetRandomStreamSeed` (`self.RNG`) _seed))
    (:`CastFailed`
      (`KismetMathLibrary.SetRandomStreamSeed` _rng (* _year _month _day _hour _minute _second _millisecond))))
  (bind _output_get (set `local.X` (`KismetMathLibrary.RandomIntegerFromStream` 5 _rng)))
  (`GenericDungeon.SetStartTile` (`self.ActiveDungeon`) _output_get 0)
  (if (and (< _y 6) _returnvalue) :!label _label
    (switch `int` (`KismetMathLibrary.RandomIntegerFromStream` 3 (`self.RNG`)) ; 1 - Up\n2 - Right\n3 - Down
      (:`0`
        (if (`.ReturnValue` (`GenericDungeon.GetTile` (`self.ActiveDungeon`) (+ (`local.X`) 1) (`local.Y`)))
          (`GenericDungeon.SetTile` (`self.ActiveDungeon`) _x_4 _y_4 (make `GenericTile` true _south_3 _east_3 _west_3))
          (`GenericDungeon.SetTile` (`self.ActiveDungeon`) _returnvalue_4 _y_4 (make `GenericTile` _north_6 true _east_6 _west_5))
          (`self.PrintDirection` _x_4 _y_4 _returnvalue_4 _y_4 "North"
            (:`Out`
              (set `local.X` _returnvalue_4)
              (goto _label)))
          (else
            (goto _label))))
      (:`1`
        (if (and (`.Void` (break `GenericTile` _tile)) _returnvalue_5)
          (`GenericDungeon.SetTile` (`self.ActiveDungeon`) _x _y_2 (make `GenericTile` _north_2 _south_2 true _west_2))
          (`KismetSystemLibrary.PrintString` (`KismetStringLibrary.Concat_StrStr` "Giving " (`KismetStringLibrary.Conv_IntToString` _x) (`KismetStringLibrary.Conv_IntToString` _returnvalue_3) " West Exit"))
          (`GenericDungeon.SetTile` (`self.ActiveDungeon`) _x _returnvalue_3 (make `GenericTile` _north_5 _south_5 _east_5 true))
          (`self.PrintDirection` _x_3 (`local.Y`) _x_3 _returnvalue_3 "East"
            (:`Out`
              (if (>= _returnvalue_3 5)
                _
                (else
                  (set `local.Y` _returnvalue_3)
                  (goto _label))))))
        (`KismetSystemLibrary.PrintString` (`KismetStringLibrary.Concat_StrStr` "Setting Goal tile" (`KismetStringLibrary.Conv_IntToString` (`local.X`)) (`KismetStringLibrary.Conv_IntToString` (`local.Y`))))
        (`GenericDungeon.SetGoalTile` (`self.ActiveDungeon`) (`local.X`) (- (`local.Y`) 1))
        (set `local.Y` (+ _y_2 1))
        (goto _label))
      (:`2`
        (if (`.ReturnValue` (`GenericDungeon.GetTile` (`self.ActiveDungeon`) (- (`local.X`) 1) (`local.Y`)))
          (`GenericDungeon.SetTile` (`self.ActiveDungeon`) _x_2 _y_3 (make `GenericTile` _north true _east _west))
          (`GenericDungeon.SetTile` (`self.ActiveDungeon`) _returnvalue_2 _y_3 (make `GenericTile` true _south_4 _east_4 _west_4))
          (`self.PrintDirection` _x_2 _y_3 _returnvalue_2 _y_3 "South"
            (:`Out`
              (set `local.X` _returnvalue_2)
              (goto _label)))
          (else
            (goto _label)))))
    (else
      (`KismetSystemLibrary.PrintString` (`KismetStringLibrary.Concat_StrStr` "Closing Loop" " y: " (`KismetStringLibrary.Conv_IntToString` _y) " !OOB: " (`KismetStringLibrary.Conv_BoolToString` _returnvalue)))
      (`GenericDungeon.SetGoalTile` (`self.ActiveDungeon`) (`local.X`) (- (`local.Y`) 1))
      (return))))

(fn `SurroundWithClosed`
  (for _index (range -1 6)
    ;[1 1 1] West Column
    (`self.RenderTile` _index -1 (make `GenericTile` false false false false false))
    ;[1 1 1] South Row
    (`self.RenderTile` -1 _index (make `GenericTile` false false false false false))
    ;[1 1 1] North Row
    (`self.RenderTile` 5 _index (make `GenericTile` false false false false false))
    ;[1 1 1] EastColumn
    (`self.RenderTile` _index 5 (make `GenericTile` false false false false false)))
  (return))

(fn `TestDungeonGeneration`
  (`GenericDungeon.SetTile` (`self.ActiveDungeon`) 0 0 (make `GenericTile` false false true))
  (`GenericDungeon.SetTile` (`self.ActiveDungeon`) 0 1 (make `GenericTile` true false false true))
  (`GenericDungeon.SetTile` (`self.ActiveDungeon`) 1 1 (make `GenericTile` true true))
  (`GenericDungeon.SetTile` (`self.ActiveDungeon`) 2 1 (make `GenericTile` false true true))
  (`GenericDungeon.SetTile` (`self.ActiveDungeon`) 2 2 (make `GenericTile` false false true true))
  (`GenericDungeon.SetTile` (`self.ActiveDungeon`) 2 3 (make `GenericTile` false false true true))
  (`GenericDungeon.SetTile` (`self.ActiveDungeon`) 2 4 (make `GenericTile` true false false true))
  (`GenericDungeon.SetTile` (`self.ActiveDungeon`) 3 4 (make `GenericTile` true true))
  (`GenericDungeon.SetTile` (`self.ActiveDungeon`) 4 4 (make `GenericTile` false true))
  (return))

(fn `UserConstructionScript`)
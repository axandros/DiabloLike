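; DMapInstance is a Blueprint that supplies seed values through GetNextSeed.
; The function multiplies the current date and time components, from year down to millisecond, so the seed is clock-based and becomes zero whenever any component is zero.
; An unconnected branch that would step through SeedList with a wrapping SeedIndex remains in the graph but never runs.
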(fn `GetNextSeed`
  (returns (Seed :type Integer))
  (bind (_year _month _day _hour _minute _second _millisecond) (`KismetMathLibrary.BreakDateTime` (`KismetMathLibrary.Now`)))
  (return (* _year _month _day _hour _minute _second _millisecond)))